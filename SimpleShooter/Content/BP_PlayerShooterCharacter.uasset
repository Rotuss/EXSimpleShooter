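; Player shooter character Blueprint that adds an intro sound and a camera zoom toggle on top of its parent class.
; On BeginPlay it calls the parent, then plays the intro sound at the character's location.
; Pressing ZoomInOut flips a zoom flag and snaps the spring arm length between close and far distances, without interpolation.
; Tick, overlap and construction script hold no custom logic.
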(event EventBeginPlay
  (|CallParentFunction)
  (Audio|PlaySoundatLocation "/Game/AssetPacks/GameDevTV/VoiceOvers/Intro.Intro" (Transformation|GetActorLocation) "0, 0, 0" 1.0 1.0 0.0 0 0 0 0))

(event Collision|EventActorBeginOverlap
  (params (OtherActor :type Actor%20Object%20Reference))
  (|CallParentFunction OtherActor) ; 지금 이 노드는 비활성 상태입니다. \n핀을 끌어서 다른 노드를 연결하면 활성화됩니다.
)

(event EventTick
  (params (DeltaSeconds :type Float%20%28single-precision%29))
  (|CallParentFunction DeltaSeconds) ; 지금 이 노드는 비활성 상태입니다. \n핀을 끌어서 다른 노드를 연결하면 활성화됩니다.
)

(event Input|ActionEvents|InputActionZoomInOut
  (params (Key :type Key%20Structure :default "None"))
  (bind _springarm (Variables|Default|GetSpringArm))
  (:Pressed
    (bind _output_get (Variables|Default|SetIsZoomIn (not (Variables|Default|GetIsZoomIn))))
    (if _output_get
      (Variables|/Script/Engine.SpringArmComponent|SetTargetArmLength _springarm 3e+01)
      (else
        (Variables|/Script/Engine.SpringArmComponent|SetTargetArmLength _springarm 3e+02)))))

(fn ConstructionScript
  (|CallParentFunction))